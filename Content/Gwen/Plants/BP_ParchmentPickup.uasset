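; BP_ParchmentPickup is a parchment pickup actor with color-tinted Niagara effects and a colored sphere mesh.
; The construction script pushes Color01 into the Niagara component and Color02 into the sphere's material Color parameter.
; On destruction it spawns the DestroyedFX Niagara system at the Bottom component's location, tinted with Color01.
; The graphs hold no overlap or collection logic of their own.
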(event `self.ReceiveBeginPlay`)

(event `self.ReceiveDestroyed`
  (bind _returnvalue (`NiagaraFunctionLibrary.SpawnSystemAtLocation` (`self.Destroyed_FX`) (`SceneComponent.K2_GetComponentLocation` (`self.Bottom`))))
  (`FXSystemComponent.SetColorParameter` _returnvalue "Color01" (`self.Color01`)))

(fn `UserConstructionScript`
  (`FXSystemComponent.SetColorParameter` (`self.Niagara`) "Color01" (`self.Color01`))
  (`MeshComponent.SetVectorParameterValueOnMaterials` (`self.Sphere`) "Color" (`KismetMathLibrary.Conv_LinearColorToVector` (`self.Color02`))))