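; BP_OscilatorComponent is a component that continuously bobs target scene components up and down along their relative Z axis.
; On BeginPlay it waits for targets supplied through SetTargets, caches their relative locations, then offsets them every frame in a zero-delay loop.
; The offset is a sine wave scaled by Speed and Scale, with the curve input switched off.
; Sync selects a shared zero start time; otherwise each instance gets a random phase.
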(event `self.ReceiveBeginPlay`
  (bind _returnvalue (* (- (`KismetSystemLibrary.GetGameTimeInSeconds`) (`self.StartTime`)) (`self.Speed`)))
  (set `self.StartTime` (`KismetMathLibrary.SelectFloat` 0.0 (+ (`KismetSystemLibrary.GetGameTimeInSeconds`) (`KismetMathLibrary.RandomFloatInRange` 0.0 6.28)) (`self.Sync?`)))
  (`/Game/Libraries/Library_Components.Wait Until` (> (`KismetArrayLibrary.Array_Length` (`self.Targets`)) 0)
    (:`Completed`
      (for _array_element (`self.Targets`)
        (`KismetArrayLibrary.Array_Add` (`self.TargetLocations`) (`SceneComponent.RelativeLocation` _array_element)))
      (for (_array_element_2 _array_index) (`self.Targets`) :!label _label
        (bind (_output_x _output_y _output_z) (`KismetMathLibrary.BreakVector` (`|GetArrayItem` (`self.TargetLocations`) _array_index)))
        (`SceneComponent.K2_SetRelativeLocation` _array_element_2 (`KismetMathLibrary.MakeVector` _output_x _output_y (+ _output_z (* (`self.Scale`) (`KismetMathLibrary.SelectFloat` (`CurveFloat.GetFloatValue` (`self.Curve`) _returnvalue) (`KismetMathLibrary.Sin` _returnvalue)) 10.0))) false false))
      (`KismetSystemLibrary.Delay` 0.0) ; (wait-one-frame)
      (goto _label))))

(event `Set Targets`
  (params (`New Targets` :type "Array of SceneComponent Object Reference"))
  (set `self.Targets` `New Targets`))