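; Player controller for Gwen that turns input into gameplay ability events and manages the player's HUD widgets.
; Left click records the world point under the cursor and sends a test event, while E and R send plant-seed and harvest-plant gameplay events to the pawn.
; BeginPlay adds a test HUD whose seed hotbar binds to the character.
; Possession adds the gameplay HUD and reveals its restart button when the pawn is destroyed.
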(event `Key|LeftMouseButton`
  (params (Key :type "Key Structure"))
  (:`Pressed`
    (set `self.Last Click Location` (`.ImpactPoint` (`GameplayStatics.BreakHitResult` (`self.GetHitResultUnderCursorByChannel` "TraceTypeQuery1"))))
    (`AbilitySystemBlueprintLibrary.SendGameplayEventToActor` (`GameplayStatics.GetPlayerPawn` 0) (struct :`TagName` "TestTag"))))

(event `self.ReceiveBeginPlay`
  (bind _returnvalue (`|CreateWidget` "/Game/Gwen/UI/WB_DamenTestHUD.WB_DamenTestHUD_C"))
  (`UserWidget.AddToViewport` _returnvalue 0)
  (`/Game/Gwen/UI/Hotbar/WB_SeedHotbar.Initialize With Character` (`/Game/Gwen/UI/WB_DamenTestHUD.WB_SeedHotbar` _returnvalue) (cast `/Game/ThirdPersonCPP/Blueprints/ThirdPersonCharacter` (`GameplayStatics.GetPlayerPawn` 0) :!pure true)))

(event `Key|E`
  (params (Key :type "Key Structure"))
  (:`Pressed`
    (`AbilitySystemBlueprintLibrary.SendGameplayEventToActor` (`GameplayStatics.GetPlayerPawn` 0) (struct :`TagName` "Ability.PlantSeed"))))

(event `Key|R`
  (params (Key :type "Key Structure"))
  (:`Pressed`
    (`AbilitySystemBlueprintLibrary.SendGameplayEventToActor` (`GameplayStatics.GetPlayerPawn` 0) (struct :`TagName` "Ability.HarvestPlant"))))

(event `self.ReceivePossess`
  (params (PossessedPawn :type "Pawn Object Reference"))
  (add `self.OnDestroyed` PossessedPawn (delegate `ShowDeathWidget`))
  (bind _returnvalue (`|CreateWidget` "/Game/Gwen/UI/WB_GameplayHUD.WB_GameplayHUD_C" self))
  (set `self.GameplayWidget` _returnvalue)
  (`UserWidget.AddToViewport` _returnvalue 0))

(event `ShowDeathWidget` :!signature `self.OnDestroyed`
  (params (DestroyedActor :type "Actor Object Reference"))
  (`Widget.SetVisibility` (`/Game/Gwen/UI/WB_GameplayHUD.Button_Restart_Game` (`self.GameplayWidget`)) "Visible"))

(fn `UserConstructionScript`)