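; BP_EpicCharacter is an enemy character that chases the player's ThirdPersonCharacter and ragdolls on death.
; On BeginPlay it issues a simple AI move toward the first ThirdPersonCharacter found and binds itself to its WB_DamenHealthBar widget.
; When health reaches zero, the mesh simulates physics while movement and capsule collision are disabled.
; A delayed destroy exists but is unconnected, so nothing here removes the body.
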(event `self.ReceiveBeginPlay`
  (`|ExecutionSequence`
    (:`then_0`
      (bind _outactors (`GameplayStatics.GetAllActorsOfClass` "/Game/ThirdPersonCPP/Blueprints/ThirdPersonCharacter.ThirdPersonCharacter_C"))
      (if (`KismetArrayLibrary.Array_IsValidIndex` _outactors)
        (bind _output (`|GetArrayItem` _outactors))
        (`/Engine/EditorBlueprintResources/StandardMacros.IsValid` _output
          (:`Is Valid`
            (bind _output_get (set `self.Target` _output))
            (`AIBlueprintHelperLibrary.SimpleMoveToActor` (`AIBlueprintHelperLibrary.GetAIController` self) _output_get)))))
    (:`then_1`
      (bind _aswb_damen_health_bar (cast `/Game/Gwen/UI/WB_DamenHealthBar` (`WidgetComponent.GetUserWidgetObject` (`self.HealthBar`))))
      (`/Game/Gwen/UI/WB_DamenHealthBar.Set Actor` _aswb_damen_health_bar self))))

(event `self.BP_OnHealthChanged`
  (params (Health :type "Float (single-precision)") (OldHealth :type "Float (single-precision)"))
  (if (<= Health 0.0)
    (`PrimitiveComponent.SetSimulatePhysics` (`self.Mesh`) true)
    (`CharacterMovementComponent.DisableMovement` (`self.CharacterMovement`))
    (`PrimitiveComponent.SetCollisionEnabled` (`self.CapsuleComponent`) "NoCollision")))

(fn `UserConstructionScript`)