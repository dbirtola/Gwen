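; GA_HarvestPlant is a gameplay ability that lets the third-person character harvest a nearby planter.
; On activation it runs a sphere overlap using the character's InteractionSphere location and radius, filtered to WorldDynamic Planter actors.
; The first overlapped planter is told to harvest if fully grown, with the owning actor passed in, then the ability ends.
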(event `self.K2_ActivateAbility`
  (bind _asthird_person_character (cast `/Game/ThirdPersonCPP/Blueprints/ThirdPersonCharacter` (`self.GetOwningActorFromActorInfo`)))
  (bind _interaction_sphere (`/Game/ThirdPersonCPP/Blueprints/ThirdPersonCharacter.Interaction Sphere` _asthird_person_character))
  (bind _outactors (`KismetSystemLibrary.SphereOverlapActors` (`SceneComponent.K2_GetComponentLocation` _interaction_sphere) (`SphereComponent.SphereRadius` _interaction_sphere) (`|MakeArray` "ObjectTypeQuery2" :!type "EObjectTypeQuery Enum") "/Game/Gwen/Plants/Planter.Planter_C"))
  (bind _asplanter (cast `/Game/Gwen/Plants/Planter` (`|GetArrayItem` _outactors)))
  (`/Game/Gwen/Plants/Planter.HarvestIfFullyGrown` _asplanter (`self.GetOwningActorFromActorInfo`))
  (`self.K2_EndAbility`))