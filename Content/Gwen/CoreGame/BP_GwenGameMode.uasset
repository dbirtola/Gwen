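; Game mode for a day/night enemy-wave game with a plant system, coordinating rounds through the level's enemy spawner and DayNightManager.
; Nightfall starts a wave and a one-shot timer for the next spawn.
; Tick runs ManageRound, which fast-forwards to day once an active round's wave is finished and no enemies have positive ability-system health, then ticks plants.
; Player death deactivates the round; reset destroys enemies and reopens the level.
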(event `self.ReceiveBeginPlay`
  (set `self.HUDClass` "/Script/GameplayAbilities.AbilitySystemDebugHUD")
  (bind _outactors (`GameplayStatics.GetAllActorsOfClass` "/Game/Gwen/Enemigo/BP_EnemySpawner.BP_EnemySpawner_C"))
  (set `self.Enemy Spawner` (`|GetArrayItem` _outactors))
  (bind _outactors_2 (`GameplayStatics.GetAllActorsOfClass` "/Script/ProjectGwen.DayNightManager"))
  (bind _output_get (set `self.DayNightManager` (`|GetArrayItem` _outactors_2)))
  (add `DayNightManager.OnNightReached` _output_get (delegate `On Nightfall`)))

(event `On Nightfall`
  (`EnemySpawner.StartWave` (`self.Enemy Spawner`) 1)
  (`KismetSystemLibrary.K2_SetTimerDelegate` (delegate `Spawn Next Enemy In Wave`) 0.3))

(event `self.ReceiveEndPlay`
  (params (EndPlayReason :type "EEndPlayReason Enum" :default "Destroyed"))
  (`PlantFunctionLibrary.PlantSystemEnd`) ; Allows the plant system to do essential cleanup
)

(event `Spawn Next Enemy In Wave`
  (`EnemySpawner.SpawnNextEnemyInWave` (`self.Enemy Spawner`)))

(event `self.ReceiveTick`
  (params (DeltaSeconds :type "Float (single-precision)"))
  (`self.ManageRound` ; Manages enemy round logic\n\nTODO: someone please correct the above assumption\nor remove this todo
    (:`exec`
      (`PlantFunctionLibrary.PlantSystemTick`) ; Optimally manages plant mechanics such as growth.\n\nTODO: add in custom parameters we can pass for effecting\nthings like global growth multiplyer and RNG variance.
    )))

(event `OnPlayerDeath`
  (set `self.bRoundActive` false))

(event `OnPlayerResetRound`
  (`|ExecutionSequence`
    (:`then_0`
      (bind _outactors (`GameplayStatics.GetAllActorsOfClass` "/Game/Gwen/Enemigo/BP_Enemy.BP_Enemy_C"))
      (for _array_element _outactors
        (`self.K2_DestroyActor` _array_element)))
    (:`then_1`
      (bind _returnvalue (`GameplayStatics.GetCurrentLevelName` true))
      (`GameplayStatics.OpenLevel` (`KismetStringLibrary.Conv_StringToName` _returnvalue)))
    (:`then_2`
      (set `self.bRoundActive` true)
      (`DayNightManager.FastForwardToDaytime` (`self.DayNightManager`)))))

(fn `GetNumberOfLivingEnemies`
  (returns (NumLivingEnemies1 :type Integer))
  (locals (NumLivingEnemies :type Integer))
  (bind _outactors (`GameplayStatics.GetAllActorsOfClass` "/Game/Gwen/Enemigo/BP_Enemy.BP_Enemy_C"))
  (if (>= (`KismetArrayLibrary.Array_Length` _outactors) 0)
    (for _array_element _outactors
      (if (> (`.ReturnValue` (`AbilitySystemBlueprintLibrary.GetFloatAttributeFromAbilitySystemComponent` (`AbilitySystemBlueprintLibrary.GetAbilitySystemComponent` _array_element) (struct :`AttributeName` "CurrentHealth" :`Attribute` "/Script/ProjectGwen.PlayerAttributeSet:CurrentHealth"))) 0.0)
        (`/Engine/EditorBlueprintResources/StandardMacros.IncrementInt` (`local.NumLivingEnemies`))))
    (return (`local.NumLivingEnemies`))
    (else
      (return 0))))

(fn `UserConstructionScript`)